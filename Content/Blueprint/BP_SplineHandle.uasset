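; BP_SplineHandle is a clickable in-game gizmo for editing a spline point or one of its tangents.
; Clicking its cube reveals axis arrows and attached tangent handles while resetting other handles.
; Clicking an arrow starts a delay loop feeding mouse delta into EditSpline until button release, repositioning tangent handles to stay mirrored.
; Tick scales the gizmo by camera distance and draws debug lines from the selected point to its tangent handles.
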(event OnBeginCursorOver(Collision_Z)
  (params (TouchedComponent :type Primitive%20Component%20Object%20Reference))
  ;[1 1 1] Move Spline Points On Z Axis
  (Components|Arrow|SetArrowColor(LinearColor) (Variables|Default|GetArrow_Z) (Utilities|Struct|MakeLinearColor 1e+02 1e+02 1e+02 0.0)))

(event OnEndCursorOver(Collision_Z)
  (params (TouchedComponent :type Primitive%20Component%20Object%20Reference))
  ;[1 1 1] Move Spline Points On Z Axis
  (Components|Arrow|SetArrowColor(LinearColor) (Variables|Default|GetArrow_Z) (Utilities|Struct|MakeLinearColor 0.0 0.0 255.0 0.0)))

(event OnEndCursorOver(Collision_X)
  (params (TouchedComponent :type Primitive%20Component%20Object%20Reference))
  ;[1 1 1] Move Spline Points On X Axis
  (Components|Arrow|SetArrowColor(LinearColor) (Variables|Default|GetArrow_X) (Utilities|Struct|MakeLinearColor 255.0 0.0 0.0 0.0)))

(event OnClicked(Collision_X)
  (params (TouchedComponent :type Primitive%20Component%20Object%20Reference) (ButtonPressed :type Key%20Structure))
  (bind _returnvalue (Game|GetPlayerController 0))
  (bind _editspline (Variables|Default|GetEditSpline))
  ;[1 1 1] Move Spline Points On X Axis
  (Variables|/Script/Engine.PlayerController|SetCurrentMouseCursor _returnvalue "GrabHandClosed")
  (Variables|/Game/Blueprint/BP_EditSpline.BP_EditSpline_C|SetIsActive _editspline true)
  (if (Variables|/Game/Blueprint/BP_EditSpline.BP_EditSpline_C|GetIsActive _editspline) :!label _label
    (CallFunction|MoveArrows (Math|Vector|MakeVector (* (.DeltaX (Class|PlayerController|GetInputMouseDelta _returnvalue)) 2e+01) 0.0 0.0))
    (Utilities|FlowControl|Delay 0.01)
    (goto _label)))

(event OnClicked(Cube)
  (params (TouchedComponent :type Primitive%20Component%20Object%20Reference) (ButtonPressed :type Key%20Structure))
  ;[1 1 1] Control handle visible
  (Variables|/Game/Blueprint/BP_EditSpline.BP_EditSpline_C|SetSelectSplinePointIndex (Variables|Default|GetEditSpline) (Variables|Default|GetSplineIndex))
  (Variables|/Script/Engine.PlayerController|SetCurrentMouseCursor (Game|GetPlayerController 0) "GrabHandClosed")
  (CallFunction|ShowHandles))

(event OnClicked(Collision_Z)
  (params (TouchedComponent :type Primitive%20Component%20Object%20Reference) (ButtonPressed :type Key%20Structure))
  (bind _returnvalue (Game|GetPlayerController 0))
  (bind _editspline (Variables|Default|GetEditSpline))
  ;[1 1 1] Move Spline Points On Z Axis
  (Variables|/Script/Engine.PlayerController|SetCurrentMouseCursor _returnvalue "GrabHandClosed")
  (Variables|/Game/Blueprint/BP_EditSpline.BP_EditSpline_C|SetIsActive _editspline true)
  (if (Variables|/Game/Blueprint/BP_EditSpline.BP_EditSpline_C|GetIsActive _editspline) :!label _label
    (CallFunction|MoveArrows (Math|Vector|MakeVector 0.0 0.0 (* (.DeltaY (Class|PlayerController|GetInputMouseDelta _returnvalue)) 2e+01)))
    (Utilities|FlowControl|Delay 0.01)
    (goto _label)))

(event OnClicked(Collision_Y)
  (params (TouchedComponent :type Primitive%20Component%20Object%20Reference) (ButtonPressed :type Key%20Structure))
  (bind _returnvalue (Game|GetPlayerController 0))
  (bind _editspline (Variables|Default|GetEditSpline))
  ;[1 1 1] Move Spline Points On Y Axis
  (Variables|/Script/Engine.PlayerController|SetCurrentMouseCursor _returnvalue "GrabHandClosed")
  (Variables|/Game/Blueprint/BP_EditSpline.BP_EditSpline_C|SetIsActive _editspline true)
  (if (Variables|/Game/Blueprint/BP_EditSpline.BP_EditSpline_C|GetIsActive _editspline) :!label _label
    (CallFunction|MoveArrows (Math|Vector|MakeVector 0.0 (* (.DeltaX (Class|PlayerController|GetInputMouseDelta _returnvalue)) 2e+01) 0.0))
    (Utilities|FlowControl|Delay 0.01)
    (goto _label)))

(event OnEndCursorOver(Collision_Y)
  (params (TouchedComponent :type Primitive%20Component%20Object%20Reference))
  ;[1 1 1] Move Spline Points On Y Axis
  (Components|Arrow|SetArrowColor(LinearColor) (Variables|Default|GetArrow_Y) (Math|Color|MakeColor 0.0 255.0 0.0 0.0)))

(event OnBeginCursorOver(Collision_Y)
  (params (TouchedComponent :type Primitive%20Component%20Object%20Reference))
  ;[1 1 1] Move Spline Points On Y Axis
  (Components|Arrow|SetArrowColor(LinearColor) (Variables|Default|GetArrow_Y) (Math|Color|MakeColor 1e+02 1e+02 1e+02 0.0)))

(event OnBeginCursorOver(Collision_X)
  (params (TouchedComponent :type Primitive%20Component%20Object%20Reference))
  ;[1 1 1] Move Spline Points On X Axis
  (Components|Arrow|SetArrowColor(LinearColor) (Variables|Default|GetArrow_X) (Utilities|Struct|MakeLinearColor 1e+02 1e+02 1e+02 0.0)))

(event EventBeginPlay
  (Utilities|FlowControl|Sequence
    (:then_0
      (bind _outactors (Actor|GetAllActorsOfClass "/Game/Blueprint/BP_SplineManager.BP_SplineManager_C"))
      (if (> (Utilities|Array|Length _outactors) 0)
        (Variables|Default|SetSplineManager (Utilities|Array|Get(acopy) _outactors))
        (else
          (Development|PrintString "BP_PlayerController:fail to find SceneManager"))))
    (:then_1
      (Rendering|Material|SetMaterial (Variables|Default|GetCube) 0 "/Game/Material/M_SplineHandle_Point.M_SplineHandle_Point") ; init cube color
    )))

(event EventTick
  (params (DeltaSeconds :type Float%20%28single-precision%29))
  (bind _outactors (Actor|GetAttachedActors))
  (bind _returnvalue (Utilities|Time|GetWorldDeltaSeconds))
  (bind _returnvalue_2 (Transformation|GetActorLocation))
  (bind _returnvalue_3 (Transformation|GetActorLocation))
  (bind _returnvalue_4 (Game|GetPlayerCameraManager 0))
  (bind _returnvalue_5 (Camera|GetCameraLocation _returnvalue_4))
  (bind _returnvalue_6 (+ _returnvalue 0.01))
  (bind _returnvalue_7 (- _returnvalue_3 _returnvalue_5))
  (bind _returnvalue_8 (Math|Vector|VectorLength _returnvalue_7))
  (bind _returnvalue_9 (/ _returnvalue_8 7e+02))
  ;[1 1 1] Draw debug line and change handles' scale as camera moving
  (Transformation|SetRelativeScale3D (Variables|Default|GetSelectPoint) (* "0.150000,0.150000,0.150000" _returnvalue_9))
  (Transformation|SetRelativeScale3D (Variables|Default|GetArrow_Y) (* "0.800000,1.000000,1.000000" _returnvalue_9))
  (Transformation|SetRelativeScale3D (Variables|Default|GetCube) (* "0.100000,0.100000,0.100000" _returnvalue_9))
  (if (Variables|Default|GetIsShowLine)
    (if (> (Utilities|Array|Length _outactors) 0)
      (Rendering|Debug|DrawDebugLine (Transformation|GetActorLocation (Utilities|Array|Get(acopy) _outactors 1)) _returnvalue_2 "(R=1.000000,G=0.000000,B=0.000000,A=1.000000)" _returnvalue_6 _returnvalue_9)
      (Rendering|Debug|DrawDebugLine _returnvalue_2 (Transformation|GetActorLocation (Utilities|Array|Get(acopy) _outactors)) "(R=1.000000,G=0.000000,B=0.000000,A=1.000000)" _returnvalue_6 _returnvalue_9))))

(event Input|MouseEvents|LeftMouseButton
  (params (Key :type Key%20Structure))
  (:Released
    (Variables|/Game/Blueprint/BP_EditSpline.BP_EditSpline_C|SetIsActive (Variables|Default|GetEditSpline) false)
    (Variables|/Script/Engine.PlayerController|SetCurrentMouseCursor (Game|GetPlayerController 0) "Default")))

(fn ConstructionScript)

(fn MoveSplinePoint
  (params (Location :type Vector))
  (bind _output_get (LocalVariables|SetTempLocation Location))
  (Transformation|SetActorLocation _output_get false false)
  (Default|SetSplinePointandMeshLocation (Variables|Default|GetEditSpline) (Variables|Default|GetSplineIndex) (LocalVariables|GetTempLocation)))

(fn MoveTangent
  (params (DeltaLocation :type Vector) (Tangent :type Vector))
  (bind _splineindex (Variables|Default|GetSplineIndex))
  (bind _editspline (Variables|Default|GetEditSpline))
  (bind _spline (Variables|/Game/Blueprint/BP_EditSpline.BP_EditSpline_C|GetSpline _editspline))
  (bind _returnvalue (Spline|GetLocationatSplinePoint _spline _splineindex "World"))
  (bind _returnvalue_2 (Spline|GetTangentatSplinePoint _spline _splineindex "World"))
  (Transformation|AddLocalOffset (Variables|Default|GetDefaultSceneRoot1) DeltaLocation false false)
  ;[1 1 1] Move edit spline points' tangents
  (Default|SetSplinePointandMeshTangent (Variables|Default|GetEditSpline) (Variables|Default|GetSplineIndex) Tangent)
  (for _array_element (Actor|GetAttachedActors (Actor|GetAttachParentActor))
    (bind _asbp_spline_handle (Utilities|Casting|CastToBP_SplineHandle _array_element))
    (if (Variables|BP_SplineHandle_C|GetIsArriveTangetPoint _asbp_spline_handle)
      (Transformation|SetActorLocation _asbp_spline_handle (- _returnvalue _returnvalue_2) false false)
      (else
        (Transformation|SetActorLocation _asbp_spline_handle (+ _returnvalue_2 _returnvalue) false false)))))

(fn SetHandleEnable
  (params (Enable :type Boolean))
  (bind _selectpoint (Variables|Default|GetSelectPoint))
  (bind _selectpoint_2 (Variables|Default|GetSelectPoint))
  (bind _cube (Variables|Default|GetCube))
  (bind _cube_2 (Variables|Default|GetCube))
  (Rendering|SetActorHiddenInGame false)
  (Collision|SetActorEnableCollision true)
  (if Enable
    (Development|SetHiddeninGame (Variables|Default|GetArrow_X) false false)
    (Collision|SetCollisionEnabled (Variables|Default|GetCollision_X) "QueryAndPhysics")
    (Development|SetHiddeninGame _selectpoint_2 false true)
    (Collision|SetCollisionEnabled _selectpoint_2 "QueryAndPhysics")
    (Collision|SetCollisionEnabled _cube_2 "NoCollision")
    (Development|SetHiddeninGame _cube_2 true true)
    (else
      (Development|SetHiddeninGame (Variables|Default|GetArrow_X) true true)
      (Collision|SetCollisionEnabled (Variables|Default|GetCollision_X) "NoCollision")
      (Development|SetHiddeninGame _selectpoint true true)
      (Collision|SetCollisionEnabled _selectpoint "NoCollision")
      (Collision|SetCollisionEnabled _cube "QueryAndPhysics")
      (Development|SetHiddeninGame _cube false true))))

(fn MoveArrows
  (params (MouseInput :type Vector))
  (LocalVariables|SetTempInput MouseInput)
  (if (Variables|Default|GetIsTangetPoint)
    (if (Variables|Default|GetIsArriveTangetPoint)
      (Variables|Default|SetTangent (- (Spline|GetTangentatSplinePoint (Variables|/Game/Blueprint/BP_EditSpline.BP_EditSpline_C|GetSpline (Variables|Default|GetEditSpline)) (Variables|Default|GetSplineIndex) "World") (LocalVariables|GetTempInput)))
      (else
        (Variables|Default|SetTangent (+ (Spline|GetTangentatSplinePoint (Variables|/Game/Blueprint/BP_EditSpline.BP_EditSpline_C|GetSpline (Variables|Default|GetEditSpline)) (Variables|Default|GetSplineIndex) "World") (LocalVariables|GetTempInput)))))
    (CallFunction|MoveTangent (LocalVariables|GetTempInput) (Variables|Default|GetTangent))
    (else
      (CallFunction|MoveSplinePoint (+ (LocalVariables|GetTempInput) (Transformation|GetWorldLocation (Variables|Default|GetDefaultSceneRoot1)))))))

(fn ShowHandles
  (bind _outactors (Actor|GetAllActorsOfClass "BP_SplineHandle_C"))
  (if (Variables|Default|GetIsTangetPoint)
    (if (> (Utilities|Array|Length _outactors) 0)
      (for _array_element _outactors
        (if (not (Variables|/Script/Engine.Actor|GetbHidden _array_element))
          (CallFunction|SetHandleEnable _array_element false)))
      (CallFunction|SetHandleEnable true))
    (elif (> (Utilities|Array|Length _outactors) 0)
      (for _array_element_2 _outactors
        (Variables|BP_SplineHandle_C|SetIsShowLine _array_element_2 false)
        (if (Variables|BP_SplineHandle_C|GetIsTangetPoint _array_element_2)
          (Rendering|SetActorHiddenInGame _array_element_2 true)
          (Collision|SetActorEnableCollision _array_element_2 false)
          (else
            (Rendering|Material|SetMaterial (Variables|BP_SplineHandle_C|GetCube _array_element_2) 0 "/Game/Material/M_SplineHandle_Point.M_SplineHandle_Point")
            (CallFunction|SetHandleEnable _array_element_2 false))))
      (Variables|Default|SetIsShowLine true)
      (CallFunction|SetHandleEnable true)
      (Rendering|Material|SetMaterial (Variables|Default|GetCube) 0 "/Game/Material/M_SplineHandle_Cube.M_SplineHandle_Cube")
      (for _array_element_3 (Actor|GetAttachedActors)
        (bind _asbp_spline_handle (Utilities|Casting|CastToBP_SplineHandle _array_element_3))
        (CallFunction|SetHandleEnable _asbp_spline_handle false)
        (Rendering|Material|SetMaterial (Variables|BP_SplineHandle_C|GetCube _asbp_spline_handle) 0 "/Game/Material/M_SplineHandle_Cube.M_SplineHandle_Cube")))))