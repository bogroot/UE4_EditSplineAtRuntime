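; BP_EditSpline is a runtime-editable spline path actor, built on BeginPlay from SplinePath point data.
; Each point spawns a BP_SplineHandle with two attached, hidden tangent handles, and spline mesh components connect neighboring points.
; Adding or deleting points reindexes the path data and rebuilds handles and meshes.
; Location and tangent setters update the spline, path data and adjacent mesh segments in place.
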(event EventBeginPlay
  (bind _splinepath (Variables|Default|GetSplinePath))
  (Utilities|IsValid (Variables|Default|GetSpline)
    (:Is%20Valid
      _)
    (:Is%20Not%20Valid
      (bind _returnvalue (AddComponent|AddSplineComponent false))
      (Variables|Default|SetSpline _returnvalue)))
  (Spline|ClearSplinePoints (Variables|Default|GetSpline) true)
  (for _array_element (.points _splinepath)
    (Spline|AddSplinePointatIndex (Variables|Default|GetSpline) (.splinepointlocation _array_element) (.splinepointindex _array_element) "World" true)
    (Spline|SetTangentatSplinePoint (Variables|Default|GetSpline) (.splinepointindex _array_element) (.splinepointtangent _array_element) "World" true))
  (Spline|SetClosedLoop (Variables|Default|GetSpline) (.bclosedpath _splinepath) true)
  (for _index (range 0 (- (Spline|GetNumberOfSplinePoints (Variables|Default|GetSpline)) 1))
    (CallFunction|CreateHandlesandSplineMesh _index)))

(event Collision|EventActorBeginOverlap
  (params (OtherActor :type Actor%20Object%20Reference)))

(event EventTick
  (params (DeltaSeconds :type Float%20%28single-precision%29)))

(fn ConstructionScript)

(fn CreateHandlesandSplineMesh
  (params (Index :type Integer))
  (bind _spline (Variables|Default|GetSpline))
  (LocalVariables|Settemp%20index Index)
  (LocalVariables|Settemp%20spline%20point%20location (Spline|GetLocationatSplinePoint (Variables|Default|GetSpline) (LocalVariables|Gettemp%20index) "World"))
  (bind _returnvalue (Game|SpawnActorfromClass "/Game/Blueprint/BP_SplineHandle.BP_SplineHandle_C" (Math|Conversions|ToTransform(Vector) (Spline|GetLocationatSplinePoint (Variables|Default|GetSpline) (LocalVariables|Gettemp%20index) "World")) "Undefined" 0 (LocalVariables|Gettemp%20index) false false self 0))
  (Default|SetHandleEnable _returnvalue false)
  (Utilities|Array|Add (Variables|Default|GetSplineLocationHandles) _returnvalue)
  (bind _returnvalue_2 (Game|SpawnActorfromClass "/Game/Blueprint/BP_SplineHandle.BP_SplineHandle_C" (Math|Conversions|ToTransform(Vector) (Math|Vector|MakeVector (- (.x (LocalVariables|Gettemp%20spline%20point%20location)) (.x (Spline|GetArriveTangentatSplinePoint (Variables|Default|GetSpline) (LocalVariables|Gettemp%20index) "World"))) (- (.y (LocalVariables|Gettemp%20spline%20point%20location)) (.y (Spline|GetArriveTangentatSplinePoint (Variables|Default|GetSpline) (LocalVariables|Gettemp%20index) "World"))) (- (.z (LocalVariables|Gettemp%20spline%20point%20location)) (.z (Spline|GetArriveTangentatSplinePoint (Variables|Default|GetSpline) (LocalVariables|Gettemp%20index) "World"))))) "Undefined" 0 (LocalVariables|Gettemp%20index) true true self 0))
  (Utilities|Array|Add (Variables|Default|GetSplineTangentHandles) _returnvalue_2)
  (Collision|SetActorEnableCollision _returnvalue_2 false)
  (Rendering|SetActorHiddenInGame _returnvalue_2 true)
  (Transformation|AttachComponentToComponent _returnvalue_2 (Variables|/Game/Blueprint/BP_SplineHandle.BP_SplineHandle_C|GetDefaultSceneRoot1 _returnvalue) "None" "KeepWorld" "KeepWorld" "KeepWorld" true)
  (bind _returnvalue_3 (Game|SpawnActorfromClass "/Game/Blueprint/BP_SplineHandle.BP_SplineHandle_C" (Math|Conversions|ToTransform(Vector) (Math|Vector|MakeVector (+ (.x (Spline|GetLeaveTangentatSplinePoint (Variables|Default|GetSpline) (LocalVariables|Gettemp%20index) "World")) (.x (LocalVariables|Gettemp%20spline%20point%20location))) (+ (.y (Spline|GetLeaveTangentatSplinePoint (Variables|Default|GetSpline) (LocalVariables|Gettemp%20index) "World")) (.y (LocalVariables|Gettemp%20spline%20point%20location))) (+ (.z (Spline|GetLeaveTangentatSplinePoint (Variables|Default|GetSpline) (LocalVariables|Gettemp%20index) "World")) (.z (LocalVariables|Gettemp%20spline%20point%20location))))) "Undefined" 0 (LocalVariables|Gettemp%20index) true false self 0))
  (Collision|SetActorEnableCollision _returnvalue_3 false)
  (Rendering|SetActorHiddenInGame _returnvalue_3 true)
  (Transformation|AttachComponentToComponent _returnvalue_3 (Variables|/Game/Blueprint/BP_SplineHandle.BP_SplineHandle_C|GetDefaultSceneRoot1 _returnvalue) "None" "KeepWorld" "KeepWorld" "KeepWorld" true)
  (if (!= (- (Spline|GetNumberOfSplinePoints (Variables|Default|GetSpline)) 1) (LocalVariables|Gettemp%20index))
    (bind _returnvalue_4 (AddComponent|AddSplineMeshComponent false))
    (Utilities|Array|Add (Variables|Default|GetSplineMesh) _returnvalue_4)
    (SplineMesh|SetStartandEnd _returnvalue_4 (.Location (Spline|GetLocationandTangentatSplinePoint _spline (LocalVariables|Gettemp%20index) "Local")) (.Tangent (Spline|GetLocationandTangentatSplinePoint _spline (LocalVariables|Gettemp%20index) "Local")) (.Location (Spline|GetLocationandTangentatSplinePoint _spline (+ (LocalVariables|Gettemp%20index) 1) "Local")) (.Tangent (Spline|GetLocationandTangentatSplinePoint _spline (+ (LocalVariables|Gettemp%20index) 1) "Local")) true :!class /Script/Engine.SplineMeshComponent)))

(fn AddSplinePoint
  (params (Position :type Vector) (PointIndex :type Integer))
  (bind _splinepath (Variables|Default|GetSplinePath))
  (bind _splinelocationhandles (Variables|Default|GetSplineLocationHandles))
  (bind _splinemesh (Variables|Default|GetSplineMesh))
  (Utilities|FlowControl|Sequence
    (:then_0
      (Spline|AddSplinePointatIndex (Variables|Default|GetSpline) Position PointIndex "World" true)
      (Utilities|Array|Insert (.points _splinepath) (Utilities|Struct|MakeS_SplinePathPoint Position (Spline|GetTangentatSplinePoint (Variables|Default|GetSpline) PointIndex "World") 0.0 0) PointIndex)
      (for (_array_element _array_index) (.points _splinepath)
        (Utilities|Array|SetArrayElem (.points _splinepath) _array_index (Utilities|Struct|MakeS_SplinePathPoint (.splinepointlocation _array_element) (.splinepointtangent _array_element) (.splinepointvelocity _array_element) _array_index))))
    (:then_1
      (for _array_element_2 _splinemesh
        (Components|DestroyComponent _array_element_2))
      (Utilities|Array|Clear _splinemesh)
      (for _array_element_3 _splinelocationhandles
        (Actor|DestroyActor (Utilities|Array|Get(acopy) (Actor|GetAttachedActors _array_element_3) 1))
        (Actor|DestroyActor (Utilities|Array|Get(acopy) (Actor|GetAttachedActors _array_element_3))))
      (Utilities|Array|Clear _splinelocationhandles)
      (Utilities|Array|Clear (Variables|Default|GetSplineTangentHandles)))
    (:then_2
      (for _index (range 0 (- (Spline|GetNumberOfSplinePoints (Variables|Default|GetSpline)) 1))
        (CallFunction|CreateHandlesandSplineMesh _index)))))

(fn GetSelectPathPoint
  (params (Path%20point :type Integer))
  (bind _splinepath (Variables|Default|GetSplinePath))
  (bind _output (Utilities|Array|Get(acopy) (.points _splinepath) Path%20point))
  (if (< Path%20point 0)
    (return "0, 0, 0" "0, 0, 0" 0.0)
    (else
      (return (.splinepointlocation _output) (.splinepointtangent _output) (.splinepointvelocity _output)))))

(fn SetSelectPathPoint
  (params (Location :type Vector) (Tangent :type Vector) (Velocity :type Float%20%28single-precision%29) (PointIndex :type Integer))
  (bind _splinepath (Variables|Default|GetSplinePath))
  (if (>= PointIndex 0)
    (Default|MoveSplinePoint (Utilities|Array|Get(acopy) (Variables|Default|GetSplineLocationHandles) PointIndex) Location)
    (Default|MoveTangent (Utilities|Array|Get(acopy) (Variables|Default|GetSplineTangentHandles) PointIndex) "0, 0, 0" Tangent)
    (bind _structout (Utilities|Struct|SetmembersinS_SplinePathPoint (Utilities|Array|Get(acopy) (.points _splinepath) PointIndex) Location Tangent Velocity))
    (Utilities|Array|SetArrayElem (.points _splinepath) PointIndex _structout true)))

(fn DeleteSplinePoint
  (params (PointIndex :type Integer))
  (bind _splinepath (Variables|Default|GetSplinePath))
  (bind _splinelocationhandles (Variables|Default|GetSplineLocationHandles))
  (bind _splinemesh (Variables|Default|GetSplineMesh))
  (Utilities|FlowControl|Sequence
    (:then_0
      (Utilities|Array|RemoveIndex (.points _splinepath) PointIndex)
      (for (_array_element _array_index) (.points _splinepath)
        (bind _structout (Utilities|Struct|SetmembersinS_SplinePathPoint _array_element _array_index))
        (Utilities|Array|SetArrayElem (.points _splinepath) _array_index _structout true))
      (Spline|RemoveSplinePoint (Variables|Default|GetSpline) PointIndex true))
    (:then_1
      ;[1 1 1] Delete Current EditSpline's handles and meshes
      (for _array_element_2 _splinemesh
        (Components|DestroyComponent _array_element_2))
      (Utilities|Array|Clear _splinemesh)
      (for _array_element_3 _splinelocationhandles
        (Actor|DestroyActor (Utilities|Array|Get(acopy) (Actor|GetAttachedActors _array_element_3) 1))
        (Actor|DestroyActor (Utilities|Array|Get(acopy) (Actor|GetAttachedActors _array_element_3)))
        (Actor|DestroyActor _array_element_3))
      (Utilities|Array|Clear _splinelocationhandles)
      (Utilities|Array|Clear (Variables|Default|GetSplineTangentHandles)))
    (:then_2
      (for _index (range 0 (- (Spline|GetNumberOfSplinePoints (Variables|Default|GetSpline)) 1))
        (CallFunction|CreateHandlesandSplineMesh _index)))))

(fn SetSplinePointandMeshLocation
  (params (PointIndex :type Integer) (Location :type Vector))
  (bind _splinemesh (Variables|Default|GetSplineMesh))
  (bind _splinepath (Variables|Default|GetSplinePath))
  (bind _splinemesh_2 (Variables|Default|GetSplineMesh))
  (bind _returnvalue (Utilities|Array|Length _splinemesh_2))
  (LocalVariables|SetTempIndex PointIndex)
  (bind _structout (Utilities|Struct|SetmembersinS_SplinePathPoint (Utilities|Array|Get(acopy) (.points _splinepath) PointIndex) Location))
  (Utilities|Array|SetArrayElem (.points _splinepath) (LocalVariables|GetTempIndex) _structout true)
  (Spline|SetLocationatSplinePoint (Variables|Default|GetSpline) (LocalVariables|GetTempIndex) Location "World" true)
  (if (== (LocalVariables|GetTempIndex) 0)
    (SplineMesh|SetStartPosition (Utilities|Array|Get(acopy) _splinemesh_2) (Spline|GetLocationatSplinePoint (Variables|Default|GetSpline) (LocalVariables|GetTempIndex) "Local") true)
    (elif (== _returnvalue (LocalVariables|GetTempIndex))
      (SplineMesh|SetEndPosition (Utilities|Array|Get(acopy) (Variables|Default|GetSplineMesh) (- _returnvalue 1)) (Spline|GetLocationatSplinePoint (Variables|Default|GetSpline) (LocalVariables|GetTempIndex) "Local") true)
      (else
        (SplineMesh|SetStartPosition (Utilities|Array|Get(acopy) _splinemesh (LocalVariables|GetTempIndex)) (Spline|GetLocationatSplinePoint (Variables|Default|GetSpline) (LocalVariables|GetTempIndex) "Local") true)
        (SplineMesh|SetEndPosition (Utilities|Array|Get(acopy) _splinemesh (- (LocalVariables|GetTempIndex) 1)) (Spline|GetLocationatSplinePoint (Variables|Default|GetSpline) (LocalVariables|GetTempIndex) "Local") true)))))

(fn SetSplinePointandMeshTangent
  (params (PointIndex :type Integer) (Tangent :type Vector))
  (bind _splinemesh (Variables|Default|GetSplineMesh))
  (bind _splinemesh_2 (Variables|Default|GetSplineMesh))
  (bind _splinepath (Variables|Default|GetSplinePath))
  (bind _returnvalue (Utilities|Array|Length _splinemesh))
  (bind _output_get (LocalVariables|SetTempIndex PointIndex))
  (LocalVariables|SetTempTangent Tangent)
  (bind _structout (Utilities|Struct|SetmembersinS_SplinePathPoint (Utilities|Array|Get(acopy) (.points _splinepath) _output_get) "0, 0, 0"))
  (Utilities|Array|SetArrayElem (.points _splinepath) (LocalVariables|GetTempIndex) _structout true)
  (Spline|SetTangentatSplinePoint (Variables|Default|GetSpline) (LocalVariables|GetTempIndex) (LocalVariables|GetTempTangent) "World" true)
  (if (== (LocalVariables|GetTempIndex) 0)
    (SplineMesh|SetStartTangent (Utilities|Array|Get(acopy) _splinemesh) (Spline|GetTangentatSplinePoint (Variables|Default|GetSpline) (LocalVariables|GetTempIndex) "Local") true :!class /Script/Engine.SplineMeshComponent)
    (elif (== _returnvalue (LocalVariables|GetTempIndex))
      (SplineMesh|SetEndTangent (Utilities|Array|Get(acopy) (Variables|Default|GetSplineMesh) (- _returnvalue 1)) (Spline|GetTangentatSplinePoint (Variables|Default|GetSpline) (LocalVariables|GetTempIndex) "Local") true :!class /Script/Engine.SplineMeshComponent)
      (else
        (SplineMesh|SetStartTangent (Utilities|Array|Get(acopy) _splinemesh_2 (LocalVariables|GetTempIndex)) (Spline|GetTangentatSplinePoint (Variables|Default|GetSpline) (LocalVariables|GetTempIndex) "Local") true :!class /Script/Engine.SplineMeshComponent)
        (SplineMesh|SetEndTangent (Utilities|Array|Get(acopy) _splinemesh_2 (- (LocalVariables|GetTempIndex) 1)) (Spline|GetTangentatSplinePoint (Variables|Default|GetSpline) (LocalVariables|GetTempIndex) "Local") true :!class /Script/Engine.SplineMeshComponent)))))